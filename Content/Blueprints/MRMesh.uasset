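; MRMesh is an actor that runs the AR session for mixed-reality environment meshes, starting it on play and stopping it on end.
; It captures scene understanding when the session config enables plane detection, otherwise spatial mapping.
; Geometry updates collect valid underlying meshes while the session runs, applying a base material if rendering is enabled.
; SpatialMapping_SetVisibility toggles that material across stored meshes and prunes invalid ones.
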(event OnAddTrackedGeometry(ARTrackableNotify)
  (params (TrackedGeometry :type AR%20Tracked%20Geometry%20Object%20Reference))
  (Development|PrintString "Adding Geometry"))

(event OnUpdateTrackedGeometry(ARTrackableNotify)
  (params (TrackedGeometry :type AR%20Tracked%20Geometry%20Object%20Reference))
  (bind _returnvalue (Class|ARBlueprintLibrary|GetARSessionStatus))
  (bind _returnvalue_2 (Class|ARTrackedGeometry|GetUnderlyingMesh TrackedGeometry))
  (bind (_additionalinfo _status) (Utilities|Struct|BreakARSessionStatus _returnvalue))
  (Development|PrintString "Updating Geometry")
  (Utilities|IsValid _returnvalue_2
    (:Is%20Valid
      (if (Utilities|Enum|Equal(Enum) _status "Running")
        (Utilities|Array|AddUnique (Variables|Default|GetTracked%20Geometry) _returnvalue_2)
        (if (Variables|Default|GetSpatial%20Mapping%20Render%20Mesh)
          (Rendering|Material|SetMaterial _returnvalue_2 0 "/Game/BaseMat.BaseMat"))
        (else
          (Development|PrintString (Utilities|String|Append "ARSession ERROR:" (Utilities|String|EnumtoString _status) _additionalinfo)))))))

(event Custom|SpatialMapping_SetVisibility
  (params (Visible :type Boolean))
  (bind _tracked_geometry (Variables|Default|GetTracked%20Geometry))
  (Variables|Default|SetSpatial%20Mapping%20Render%20Mesh Visible)
  (for _array_element _tracked_geometry
    (Utilities|IsValid _array_element
      (:Is%20Valid
        (Rendering|Material|SetMaterial _array_element 0 (select (Variables|Default|GetSpatial%20Mapping%20Render%20Mesh) "/Game/BaseMat.BaseMat" 0)))
      (:Is%20Not%20Valid
        (Utilities|Array|RemoveItem _tracked_geometry _array_element)))))

(event EventBeginPlay
  (Class|ARBlueprintLibrary|StartARSession "/Game/DataAsset.DataAsset")
  (if (not (Utilities|Enum|Equal(Enum) (Class|ARSessionConfig|GetPlaneDetectionMode (Class|ARBlueprintLibrary|GetSessionConfig)) "None"))
    (Class|ARBlueprintLibrary|ToggleARCapture true "SceneUnderstanding")
    (Development|PrintString "Scene Understanding ON" true true "(R=0.203919,G=1.000000,B=0.000000,A=1.000000)" 4.0)
    (else
      (Class|ARBlueprintLibrary|ToggleARCapture true "SpatialMapping")
      (Development|PrintString "Spatial Mapping ON" true true "(R=0.203919,G=1.000000,B=0.000000,A=1.000000)" 4.0))))

(event Collision|EventActorBeginOverlap
  (params (OtherActor :type Actor%20Object%20Reference)))

(event EventTick
  (params (DeltaSeconds :type Float%20%28single-precision%29)))

(event EventEndPlay
  (params (EndPlayReason :type EEndPlayReason%20Enum :default "Destroyed"))
  (Class|ARBlueprintLibrary|StopARSession))

(fn ConstructionScript)