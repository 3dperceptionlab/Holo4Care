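; AR actor that scans the real environment and colors the detected meshes by what they are, such as walls, floors or furniture.
; On BeginPlay it starts an AR session and spawns an info widget, then after a delay enables Scene Understanding or, without plane detection, Spatial Mapping capture.
; Geometry updates set each mesh's material from its classification and show that class on the widget.
; EndPlay switches the capture off.
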(event OnAddTrackedGeometry(ARTrackableNotify)
  (params (TrackedGeometry :type AR%20Tracked%20Geometry%20Object%20Reference)))

(event OnUpdateTrackedGeometry(ARTrackableNotify)
  (params (TrackedGeometry :type AR%20Tracked%20Geometry%20Object%20Reference))
  (bind _returnvalue (Class|ARTrackedGeometry|GetObjectClassification TrackedGeometry))
  (bind _returnvalue_2 (Class|ARTrackedGeometry|GetUnderlyingMesh TrackedGeometry))
  (if (Utilities|IsValid _returnvalue_2)
    (CallFunction|ShowActionText (Utilities|Text|ToText(String) (Utilities|String|EnumtoString _returnvalue)))
    (switch Utilities|FlowControl|Switch|SwitchonEARObjectClassification _returnvalue
      (:Unknown
        (Rendering|Material|SetMaterial _returnvalue_2 0 "/Game/Materials/BaseMat.BaseMat"))
      (:Wall
        (Rendering|Material|SetMaterial _returnvalue_2 0 "/Game/Materials/BaseMat2.BaseMat2"))
      (:Ceiling
        (Rendering|Material|SetMaterial _returnvalue_2 0 "/Game/Materials/BaseMat3.BaseMat3"))
      (:Floor
        (Rendering|Material|SetMaterial _returnvalue_2 0 "/Game/Materials/BaseMat3.BaseMat3"))
      (:Table
        (Rendering|Material|SetMaterial _returnvalue_2 0 "/Game/Materials/BaseMat4.BaseMat4"))
      (:Seat
        (Rendering|Material|SetMaterial _returnvalue_2 0 "/Game/Materials/BaseMat4.BaseMat4"))
      (:SceneObject
        (Rendering|Material|SetMaterial _returnvalue_2 0 "/Game/Materials/BaseMat5.BaseMat5"))
      (:Door
        (Rendering|Material|SetMaterial _returnvalue_2 0 "/Game/Materials/BaseMat3.BaseMat3")))))

(event Custom|OnTimerDelay
  (if (Variables|Default|GetCanDetectPlanes)
    (Class|ARBlueprintLibrary|ToggleARCapture true "SceneUnderstanding")
    (CallFunction|ShowActionText "SCENE UNDERSTANDING")
    (else
      (Class|ARBlueprintLibrary|ToggleARCapture true "SpatialMapping")
      (CallFunction|ShowActionText "SPATIAL MAPPING"))))

(event EventBeginPlay
  (bind _returnvalue (Class|ARBlueprintLibrary|GetSessionConfig))
  (bind _returnvalue_2 (Class|ARSessionConfig|GetPlaneDetectionMode _returnvalue))
  (Class|ARBlueprintLibrary|StartARSession "/Game/DataAsset.DataAsset")
  (bind _returnvalue_3 (Game|SpawnActorfromClass "/Game/Blueprints/WidgetActorInfo.WidgetActorInfo_C" (Math|Transform|MakeTransform "60.000000,60.000000,140.000000" "0, 0, 0" "1,1,1") "Undefined" self 0))
  (Variables|Default|SetWidget%20Info _returnvalue_3)
  (CallFunction|ShowActionText "INICIADO")
  (Utilities|Time|SetTimerbyEvent (delegate Custom|OnTimerDelay) 5.0)
  (Variables|Default|SetCanDetectPlanes (or (Utilities|Enum|Equal(Enum) _returnvalue_2 "HorizontalPlaneDetection") (Utilities|Enum|Equal(Enum) _returnvalue_2 "VerticalPlaneDetection"))))

(event EventEndPlay
  (params (EndPlayReason :type EEndPlayReason%20Enum :default "Destroyed"))
  (if (Variables|Default|GetCanDetectPlanes)
    (Class|ARBlueprintLibrary|ToggleARCapture false "SceneUnderstanding")
    (else
      (Class|ARBlueprintLibrary|ToggleARCapture false "SpatialMapping"))))

(fn ConstructionScript)

(fn ShowActionText
  (params (Texto :type Text))
  (bind _aswidget_information (Utilities|Casting|CastToWidgetInformation (UserInterface|GetUserWidgetObject (Variables|/Game/Blueprints/WidgetActorInfo.WidgetActorInfo_C|GetWidget (Variables|Default|GetWidget%20Info)))))
  (Default|SetInfoText _aswidget_information Texto))